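; Drivable buggy vehicle Blueprint that passes throttle and steering input to its movement component and supports switching between in-car and exterior cameras.
; Look input rotates the active camera's spring arm with clamped pitch, and V toggles the view.
; The Driver event stores the player's controller and selects the exterior camera.
; CarToggle exits by spawning a new third-person character at the Arrow component and possessing it.
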(event EventDriver
  (params (Instigator :type Player%20Controller%20Object%20Reference))
  (Variables|Default|SetPlayerController Instigator)
  (Components|Activation|SetActive (Variables|Default|GetIncarCam) false false)
  (Components|Activation|SetActive (Variables|Default|GetOutcarCam) true false))

(event Input|ActionEvents|InputActionCarToggle
  (params (Key :type Key%20Structure))
  (bind _arrow (Variables|Default|GetArrow))
  (bind _returnvalue (Transformation|GetWorldTransform _arrow))
  (:Pressed
    (Variables|Default|SetbIsFPS false)
    (bind _returnvalue_2 (Game|SpawnActorfromClass "/Game/ThirdPersonBP/Blueprints/ThirdPersonCharacter.ThirdPersonCharacter_C" (Math|Transform|MakeTransform (.location _returnvalue) (Math|Rotator|MakeRotator 0.0 0.0 (.yaw (.rotation _returnvalue))) "1,1,1") "Undefined" 0 0))
    (Pawn|Possess (Variables|Default|GetPlayerController) _returnvalue_2)))

(event Input|AxisEvents|InputAxisMoveForward
  (params (AxisValue :type Float%20%28single-precision%29))
  (Class|WheeledVehicleMovementComponent|SetThrottleInput (Variables|Default|GetVehicleMovement) AxisValue))

(event Input|AxisEvents|InputAxisMoveRight
  (params (AxisValue :type Float%20%28single-precision%29))
  (Class|WheeledVehicleMovementComponent|SetSteeringInput (Variables|Default|GetVehicleMovement) AxisValue))

(event Input|AxisEvents|InputAxisLookUp
  (params (AxisValue :type Float%20%28single-precision%29))
  (bind _bisfps (Variables|Default|GetbIsFPS))
  (bind _springarm (Variables|Default|GetSpringArm))
  (bind _springarm1 (Variables|Default|GetSpringArm1))
  (bind _returnvalue (select _bisfps _springarm1 _springarm))
  (bind _relativerotation (Variables|/Script/Engine.SceneComponent|GetRelativeRotation _returnvalue))
  (Transformation|SetRelativeRotation _returnvalue (Math|Rotator|MakeRotator (.roll _relativerotation) (Math|Float|Clamp(Float) (+ (* AxisValue -1.0) (.pitch _relativerotation)) -8e+01 1e+01) (.yaw _relativerotation)) false false))

(event Input|AxisEvents|InputAxisLookRight
  (params (AxisValue :type Float%20%28single-precision%29))
  (bind _bisfps (Variables|Default|GetbIsFPS))
  (bind _springarm (Variables|Default|GetSpringArm))
  (bind _springarm1 (Variables|Default|GetSpringArm1))
  (bind _returnvalue (select _bisfps _springarm1 _springarm))
  (bind _relativerotation (Variables|/Script/Engine.SceneComponent|GetRelativeRotation _returnvalue))
  (Transformation|SetRelativeRotation _returnvalue (Math|Rotator|MakeRotator (.roll _relativerotation) (.pitch _relativerotation) (+ AxisValue (.yaw _relativerotation))) false false))

(event Input|KeyboardEvents|V
  (params (Key :type Key%20Structure))
  (:Pressed
    (Variables|Default|SetbIsFPS (not (Variables|Default|GetbIsFPS)))
    (Components|Activation|SetActive (Variables|Default|GetIncarCam) (Variables|Default|GetbIsFPS) false)
    (Components|Activation|SetActive (Variables|Default|GetOutcarCam) (not (Variables|Default|GetbIsFPS)) false)))

(fn ConstructionScript)